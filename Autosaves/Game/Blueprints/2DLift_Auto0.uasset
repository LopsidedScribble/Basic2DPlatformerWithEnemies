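; 2D lift actor that moves its sprite back and forth between its relative origin and EndLocation.
; A timeline lerps the sprite position, then waits StopDelay and switches between LiftForward and LiftBack to loop; nothing in this graph starts the cycle.
; The construction script previews the end position when TestEndLocation is set.
; The SafteyCollider overlap only casts to MyCharacter, with no further action.
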(event `self.SafteyCollider.OnComponentBeginOverlap`
  (params (OverlappedComponent :type "PrimitiveComponent Object Reference") (OtherActor :type "Actor Object Reference") (OtherComp :type "PrimitiveComponent Object Reference") (OtherBodyIndex :type Integer) (bFromSweep :type Boolean) (SweepResult :type "HitResult Structure (by ref)"))
  (cast `/Game/Blueprints/MyCharacter` OtherActor))

(event `LiftForward`
  (bind (_direction _lerp_alpha) (`Timeline|Lift Timeline` :!via `PlayFromStart` :!label _label)
    (:`Update`
      (`SceneComponent.K2_SetRelativeLocation` (`self.LiftSprite`) (`KismetMathLibrary.VLerp` (0.0 0.0 0.0) (`self.EndLocation`) _lerp_alpha) false false))
    (:`Finished`
      (`KismetSystemLibrary.Delay` (`self.Stop Delay`))
      (switch `ETimelineDirection` _direction
        (:`Forward`
          (`self.LiftBack`))
        (:`Backward`
          (`self.LiftForward`))))))

(event `LiftBack`
  (goto _label :!via `ReverseFromEnd`))

(fn `UserConstructionScript`
  (`SceneComponent.K2_SetRelativeLocation` (`self.LiftSprite`) (`KismetMathLibrary.SelectVector` (`self.EndLocation`) (0.0 0.0 0.0) (`self.TestEndLocation`)) false false))